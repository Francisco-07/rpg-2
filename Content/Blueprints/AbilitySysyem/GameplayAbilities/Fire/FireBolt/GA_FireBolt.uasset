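; GA_FireBolt is a Gameplay Ability that casts a fire bolt projectile in the player's aim direction.
; On activation it commits, line-traces forward from the player camera and plays the magic attack montage.
; A montage gameplay event triggers SpawnProjectile with the trace's end point, captured at activation, rather than any impact point.
; The ability ends when the montage completes, blends out, is interrupted or is cancelled.
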(event Ability|EventActivateAbility
  (bind _returnvalue (Game|GetPlayerCameraManager 0))
  (bind _returnvalue_2 (Transformation|GetActorLocation _returnvalue))
  (Ability|CommitAbility)
  ;[1 1 1] Line trace for calculatiing projectile direction MUST DO IT REUSABLE
  (bind _outhit (Collision|LineTraceByChannel _returnvalue_2 (+ _returnvalue_2 (* (Transformation|GetActorForwardVector _returnvalue) "2000.000000,2000.000000,2000.000000")) "TraceTypeQuery1" false 0 "None"))
  (|PlayMontageandWaitProxy "None" "/Game/Mannequin/Animations/Manny/AM_MagicAttack.AM_MagicAttack" 1.0 "None" false 1.0 0.0 false
    (:then
      (Ability|Tasks|WaitGameplayEvent "(TagName=\"Event.Montage.FireBolt\")" 0
        (:EventReceived
          (Class|RPGProjectileSpell|SpawnProjectile (.TraceEnd (Collision|BreakHitResult _outhit))))))
    (:OnCompleted
      (Ability|EndAbility :!label _label))
    (:OnBlendOut
      (goto _label))
    (:OnInterrupted
      (goto _label))
    (:OnCancelled
      (goto _label))))

(event Ability|EventOnEndAbility
  (params (bWasCancelled :type Boolean)))